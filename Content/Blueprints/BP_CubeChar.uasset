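; BP_CubeChar is a character Blueprint that provides basic movement and jumping.
; MoveForward and MoveRight axis inputs feed AddMovementInput along the actor's forward and right vectors, and the Jump action calls Jump on press.
; Four custom events (f_MoveForward, f_MoveBack, f_MoveLeft, f_MoveRight) apply full-scale movement in each direction, allowing movement to be triggered without axis input.
; A debug text print is left unconnected, and the construction script is empty.
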(event `f_MoveBack`
  (`self.AddMovementInput` (`self.GetActorForwardVector`) -1.0))

(event `f_MoveLeft`
  (`self.AddMovementInput` (`self.GetActorRightVector`) -1.0))

(event `f_MoveForward`
  (`self.AddMovementInput` (`self.GetActorForwardVector`)))

(event `f_MoveRight`
  (`self.AddMovementInput` (`self.GetActorRightVector`)))

(event `InputAxis|MoveRight` :consume false :overrideparent false
  (params (AxisValue :type "Float (single-precision)"))
  (`self.AddMovementInput` (`self.GetActorRightVector`) AxisValue))

(event `InputAxis|MoveForward` :consume false
  (params (AxisValue :type "Float (single-precision)"))
  (`self.AddMovementInput` (`self.GetActorForwardVector`) AxisValue))

(event `InputAction|Jump`
  (params (Key :type "Key Structure"))
  (:`Pressed`
    (`self.Jump`)))

(fn `UserConstructionScript`)