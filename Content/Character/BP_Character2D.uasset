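; BP_Character2D is a side-scrolling 2D character that runs along the world X axis and jumps.
; The MoveRight axis switches the sprite flipbook between Idle and Run and feeds movement input.
; Non-zero input flips the sprite by rotating it 180 degrees for leftward movement, so it keeps its last facing when idle.
; The Jump action calls the built-in character jump.
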(event `InputAxis|MoveRight`
  (params (AxisValue :type "Float (single-precision)"))
  (`PaperFlipbookComponent.SetFlipbook` (`self.Sprite`) (select `bool` (== AxisValue 0.0) :`false` "/Game/Character/Animations/Flipbooks/Run.Run" :`true` "/Game/Character/Animations/Flipbooks/Idle.Idle" :!type "PaperFlipbook Object Reference"))
  (`self.AddMovementInput` (1.0 0.0 0.0) AxisValue)
  (if (!= AxisValue 0.0)
    (`SceneComponent.K2_SetRelativeRotation` (`self.Sprite`) (select `bool` (> AxisValue 0.0) :`false` (struct :`Yaw` 180.0) :!type "Rotator Structure") false false)))

(event `InputAction|Jump`
  (params (Key :type "Key Structure"))
  (:`Pressed`
    (`self.Jump`)))

(fn `UserConstructionScript`)